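; Enemy character that takes a random mesh on spawn, chases the player and melee-attacks.
; ChasePlayer runs AI MoveTo, then plays a push montage whose notify sphere-traces to apply damage, restarting the chase on completion.
; Non-lethal damage knocks it back; death ragdolls it, destroys it after a delay and has BP_WaveSpawner check for remaining enemies.
; The random-wander event is deprecated.
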(event `self.ReceiveBeginPlay`
  (`self.Chase Player`)
  (`SkeletalMeshComponent.SetSkeletalMeshAsset` (`self.Mesh`) (`KismetArrayLibrary.Array_Random` (`self.Meshes`))))

(event `Wonder`
  ;[1 1 1] 敌人随机移动(弃用)
  (`|AIMoveTo` self (`NavigationSystemV1.K2_GetRandomReachablePointInRadius` (`self.K2_GetActorLocation`) 500.0 null null) null
    (:`OnSuccess`
      (`KismetSystemLibrary.Delay` 1.0)
      (`self.Wonder`))))

(event `self.ReceiveAnyDamage`
  (params (Damage :type "Float (single-precision)") (DamageType :type "DamageType Object Reference") (InstigatedBy :type "Controller Object Reference") (DamageCauser :type "Actor Object Reference"))
  ;[1 1 1] 敌人受伤
  (set `self.E_Health` (- (`self.E_Health`) Damage))
  (if (<= (`self.E_Health`) 0.0)
    (`PrimitiveComponent.SetSimulatePhysics` (`self.Mesh`) true)
    ;[1 1 1] 死亡销毁，生成下一波
    (set `self.Can Attack` false)
    (`CharacterMovementComponent.DisableMovement` (`self.CharacterMovement`))
    (`KismetSystemLibrary.Delay` 2.0)
    (`self.K2_DestroyActor`)
    (bind _returnvalue (`GameplayStatics.GetActorOfClass` "/Game/BluePrints/BP_WaveSpawner.BP_WaveSpawner_C"))
    (`/Game/BluePrints/BP_WaveSpawner.Check for Enemies` _returnvalue)
    (else
      (`self.LaunchCharacter` (+ (* (`self.GetActorForwardVector`) -300.0) (* (`self.GetActorUpVector`) 100.0))))))

(event `Chase Player`
  (bind _attack_track_pos (`self.Attack Track Pos`))
  (bind _returnvalue (`SceneComponent.K2_GetComponentLocation` _attack_track_pos))
  ;[1 1 1] 敌人追着主角攻击
  (`|AIMoveTo` self (0.0 0.0 0.0) (`GameplayStatics.GetPlayerCharacter` 0)
    (:`OnSuccess`
      (if (`self.Can Attack`)
        (`|PlayMontage` (`self.Mesh`) "/Game/Characters/Mannequin_UE4/OurAnimations/Push_Montage.Push_Montage"
          (:`then`
            (set `self.Can Attack` false)
            ;[1 1 1] 受击音效
            (`GameplayStatics.PlaySoundAtLocation` "/Game/Audio/MS_DamageGrunt.MS_DamageGrunt" (`self.K2_GetActorLocation`) (struct) 1.0 1.0 0.0 null null null null))
          (:`OnCompleted`
            (set `self.Can Attack` true)
            (`self.Chase Player`))
          (:`OnNotifyBegin`
            (bind (_outhit _returnvalue_2) (`KismetSystemLibrary.SphereTraceSingleForObjects` _returnvalue (+ _returnvalue (* (`SceneComponent.GetForwardVector` _attack_track_pos) 100.0)) 25.0 (`|MakeArray` "ObjectTypeQuery3" :!type "EObjectTypeQuery Enum")))
            (if _returnvalue_2
              (`GameplayStatics.ApplyDamage` (`.HitActor` (`GameplayStatics.BreakHitResult` _outhit)) 10.0))))))))

(fn `UserConstructionScript`)